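; Legacy Warrok enemy character that chases and attacks the hero with a hammer spawned into its right hand.
; AI sight perception starts or stops pursuit, while Tick feeds movement speed to AB_Warrok.
; A short forward trace finding the hero randomly triggers one of two attack animation states and briefly halts movement.
; Only BP_Sword damage lowers health, playing a hit state or a death state followed by delayed destruction of Warrok and hammer.
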(event `self.ReceiveBeginPlay`
  (bind _returnvalue (`|SpawnActorFromClass` "/Game/Pangaea/Weapons/Hammer/BP_Hammer.BP_Hammer_C" (`self.GetTransform`) "AlwaysSpawn" "MultiplyWithRoot" null null))
  (bind _output_get (set `self.Weapon` _returnvalue))
  (`self.K2_AttachToComponent` _output_get (`self.Mesh`) "RightHandSocket" "SnapToTarget" "SnapToTarget" "SnapToTarget" true))

(event `self.ReceiveTick`
  (params (DeltaSeconds :type "Float (single-precision)"))
  (bind _returnvalue (`self.GetMovementComponent`))
  (bind _returnvalue_2 (`self.K2_GetActorLocation`))
  (bind _animinst (`self.GetAnimInst`))
  (bind _returnvalue_3 (`KismetMathLibrary.RandomFloat`))
  (if (> (`self.Health`) 0.0)
    (bind _returnvalue_4 (message `NavMovementInterface.GetVelocityForNavMovement` _returnvalue))
    (bind _returnvalue_5 (message `NavMovementInterface.GetMaxSpeedForNavMovement` _returnvalue))
    (set `/Game/Pangaea/Characters/Warrok/AB_Warrok.Speed` (* (/ (`KismetMathLibrary.VSize` _returnvalue_4) _returnvalue_5) 100.0) (`self.GetAnimInst`))
    (bind (_outhit _returnvalue_6) (`KismetSystemLibrary.LineTraceSingleForObjects` _returnvalue_2 (+ _returnvalue_2 (* (`self.GetActorForwardVector`) 150.0)) (`self.Object Types`) true))
    (if _returnvalue_6
      (bind _asbp_hero (cast `/Game/Pangaea/Characters/Hero/BP_Hero` (`.HitActor` (`GameplayStatics.BreakHitResult` _outhit))))
      (if (== (`/Game/Pangaea/Characters/Warrok/AB_Warrok.AnimState` _animinst) 0)
        (if (< _returnvalue_3 0.1)
          (set `/Game/Pangaea/Characters/Warrok/AB_Warrok.AnimState` 11 _animinst)
          (`Controller.StopMovement` (`AIBlueprintHelperLibrary.GetAIController` self) :!label _label)
          (`KismetSystemLibrary.Delay` 1.5)
          (`AIBlueprintHelperLibrary.SimpleMoveToActor` (`AIBlueprintHelperLibrary.GetAIController` self) _asbp_hero)
          (elif (< _returnvalue_3 0.15)
            (set `/Game/Pangaea/Characters/Warrok/AB_Warrok.AnimState` 12 _animinst)
            (goto _label)))))))

(event `self.ReceiveAnyDamage`
  (params (Damage :type "Float (single-precision)") (DamageType :type "DamageType Object Reference") (InstigatedBy :type "Controller Object Reference") (DamageCauser :type "Actor Object Reference"))
  (bind _animinst (`self.GetAnimInst`))
  (cast `/Game/Pangaea/Weapons/Sword/BP_Sword` DamageCauser)
  (bind _output_get (set `self.Health` (`KismetMathLibrary.FMax` (- (`self.Health`) Damage))))
  (`Controller.StopMovement` (`AIBlueprintHelperLibrary.GetAIController` self))
  (if (> _output_get 0.0)
    (set `/Game/Pangaea/Characters/Warrok/AB_Warrok.AnimState` 2 _animinst)
    (`KismetSystemLibrary.Delay` 1.5)
    (`AIBlueprintHelperLibrary.SimpleMoveToActor` (`AIBlueprintHelperLibrary.GetAIController` self))
    (else
      (set `/Game/Pangaea/Characters/Warrok/AB_Warrok.AnimState` 3 _animinst)
      (`KismetSystemLibrary.Delay` 5.0)
      (`self.K2_DestroyActor`)
      (`self.K2_DestroyActor` (`self.Weapon`)))))

(event `self.AIPerception.OnTargetPerceptionUpdated`
  (params (Actor :type "Actor Object Reference") (Stimulus :type "AIStimulus Structure"))
  (bind _returnvalue (`AIBlueprintHelperLibrary.GetAIController` self))
  (bind _returnvalue_2 (`AIPerceptionSystem.GetSenseClassForStimulus` Stimulus))
  (if (== _returnvalue_2 "/Script/AIModule.AISense_Sight")
    (if (`.bSuccessfullySensed` (break `AIStimulus` Stimulus))
      (cast `/Game/Pangaea/Characters/Hero/BP_Hero` Actor)
      (`AIBlueprintHelperLibrary.SimpleMoveToActor` _returnvalue Actor)
      (else
        (`Controller.StopMovement` _returnvalue)))))

(fn `GetAnimInst`
  (returns (AnimInst :type "/Game/Pangaea/Characters/Warrok/AB_Warrok Object Reference"))
  (bind _asab_warrok (cast `/Game/Pangaea/Characters/Warrok/AB_Warrok` (`SkeletalMeshComponent.GetAnimInstance` (`self.Mesh`))))
  (return _asab_warrok))

(fn `UserConstructionScript`)