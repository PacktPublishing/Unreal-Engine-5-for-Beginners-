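; BP_Boss is an AI-driven boss enemy that spawns a BP_Axe into its right hand and feeds normalized movement speed to its AB_Boss animation instance.
; AI perception sets or clears the blackboard's PlayerTarget as it senses BP_Hero.
; In certain animation states, BP_Sword hits reduce health, stop movement and set Hit/Killed blackboard keys.
; Damage events in those states also register the living boss with HUD widgets, or clear it at zero health.
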(event `self.ReceiveBeginPlay`
  (bind _returnvalue (`|SpawnActorFromClass` "/Game/Pangaea/Weapons/Axe/BP_Axe.BP_Axe_C" (`self.GetTransform`) "AlwaysSpawn" "MultiplyWithRoot" null null))
  (bind _output_get (set `self.Weapon` _returnvalue))
  (`self.K2_AttachToComponent` _output_get (`self.Mesh`) "RightHandSocket" "SnapToTarget" "SnapToTarget" "SnapToTarget" true)
  (set `self.Health` (`self.MaxHealth`)))

(event `self.ReceiveTick`
  (params (DeltaSeconds :type "Float (single-precision)"))
  (bind _returnvalue (`self.GetMovementComponent`))
  (if (> (`self.Health`) 0.0)
    (bind _returnvalue_2 (message `NavMovementInterface.GetVelocityForNavMovement` _returnvalue))
    (bind _returnvalue_3 (message `NavMovementInterface.GetMaxSpeedForNavMovement` _returnvalue))
    (set `/Game/Pangaea/Characters/Boss/AB_Boss.Speed` (* (/ (`KismetMathLibrary.VSize` _returnvalue_2) _returnvalue_3) 100.0) (`self.GetAnimInst`))))

(event `self.AIPerception.OnTargetPerceptionInfoUpdated`
  (params (UpdateInfo :type "ActorPerceptionUpdateInfo Structure (by ref)"))
  (bind (_targetid _target _stimulus) (break `ActorPerceptionUpdateInfo` UpdateInfo))
  (bind _returnvalue (`AIBlueprintHelperLibrary.GetBlackboard` (`AIBlueprintHelperLibrary.GetAIController` self)))
  (if (`.bSuccessfullySensed` (break `AIStimulus` _stimulus))
    (bind _asbp_hero (cast `/Game/Pangaea/Characters/Hero/BP_Hero` _target)
      (:`then`
        (`BlackboardComponent.SetValueAsObject` _returnvalue "PlayerTarget" _asbp_hero))
      (:`CastFailed`
        (`BlackboardComponent.ClearValue` _returnvalue "PlayerTarget" :!label _label)))
    (else
      (goto _label))))

(event `self.ReceiveAnyDamage`
  (params (Damage :type "Float (single-precision)") (DamageType :type "DamageType Object Reference") (InstigatedBy :type "Controller Object Reference") (DamageCauser :type "Actor Object Reference"))
  (bind _returnvalue (`AIBlueprintHelperLibrary.GetAIController` self))
  (bind _animstate (`/Game/Pangaea/Characters/Boss/AB_Boss.AnimState` (`self.GetAnimInst`)))
  (bind _returnvalue_2 (`AIBlueprintHelperLibrary.GetBlackboard` _returnvalue))
  (if (or (or (== _animstate 0) (== _animstate 11)) (== _animstate 12))
    (`|ExecutionSequence`
      (:`then_0`
        (cast `/Game/Pangaea/Weapons/Sword/BP_Sword` DamageCauser)
        (bind _output_get (set `self.Health` (`KismetMathLibrary.FMax` (- (`self.Health`) Damage))))
        (`Controller.StopMovement` _returnvalue)
        (`BlackboardComponent.SetValueAsBool` _returnvalue_2 "Hit" true)
        (`BlackboardComponent.SetValueAsBool` _returnvalue_2 "Killed" (<= _output_get 0.0)))
      (:`then_1`
        (bind _foundwidgets (`WidgetBlueprintLibrary.GetAllWidgetsOfClass` "/Game/Pangaea/UI/HUD.HUD_C"))
        (for _array_element _foundwidgets
          (if (> (`self.Health`) 0.0)
            (set `/Game/Pangaea/UI/HUD.EnemyBoss` self _array_element)
            (else
              (set `/Game/Pangaea/UI/HUD.EnemyBoss` null _array_element))))))))

(fn `GetAnimInst`
  (returns (AnimationInstance :type "/Game/Pangaea/Characters/Boss/AB_Boss Object Reference"))
  (bind _asab_boss (cast `/Game/Pangaea/Characters/Boss/AB_Boss` (`SkeletalMeshComponent.GetAnimInstance` (`self.Mesh`))))
  (return _asab_boss))

(fn `IsInLocomotionState`
  (returns (Result :type Boolean))
  (return (== (`/Game/Pangaea/Characters/Boss/AB_Boss.AnimState` (`self.GetAnimInst`)) 0)))

(fn `UserConstructionScript`)