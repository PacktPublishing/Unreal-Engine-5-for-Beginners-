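; BP_Hammer is the hammer weapon carried by the Warrok character, dealing damage to actors it overlaps.
; On overlap it ignores the actor it is attached to, then casts that parent to BP_Warrok and reads its AB_Warrok anim instance.
; Fixed damage applies only while the animation state is one of two specific values, so the hammer hurts only during those states.
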(event `self.ReceiveActorBeginOverlap`
  (params (OtherActor :type "Actor Object Reference"))
  (bind _returnvalue (`self.GetAttachParentActor`))
  (if (!= OtherActor _returnvalue)
    (bind _asbp_warrok (cast `/Game/Pangaea/Characters/Warrok/BP_Warrok` _returnvalue))
    (bind _asab_warrok (cast `/Game/Pangaea/Characters/Warrok/AB_Warrok` (`SkeletalMeshComponent.GetAnimInstance` (`Character.Mesh` _asbp_warrok))))
    (bind _animstate (`/Game/Pangaea/Characters/Warrok/AB_Warrok.AnimState` _asab_warrok))
    (if (or (== _animstate 11) (== _animstate 12))
      (`GameplayStatics.ApplyDamage` OtherActor 80.0 null self))))

(fn `UserConstructionScript`)