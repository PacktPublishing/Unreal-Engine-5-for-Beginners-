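; BP_Mission runs a mission made of ordered objectives and handles the win state.
; On BeginPlay it prints the goal and, after a short delay, shows it on a HUD widget.
; Tick polls the Objectives array, activating the first incomplete one or marking the mission completed when none remain.
; On completion, a DoOnce sets the HUD game-over text to a win message, then loads the main menu after a delay.
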(event `self.ReceiveBeginPlay`
  (bind _goal (`self.Goal`))
  (`KismetSystemLibrary.PrintString` _goal true true (struct :`G` 0.66 :`B` 1.0 :`A` 1.0) 15.0)
  (`KismetSystemLibrary.Delay` 0.2)
  (bind _foundwidgets (`WidgetBlueprintLibrary.GetAllWidgetsOfClass` "/Game/Pangaea/UI/HUD1.HUD1_C"))
  (`/Game/Pangaea/UI/HUD1.ShowMissionOrObjective` (`|GetArrayItem` _foundwidgets) _goal))

(event `self.ReceiveTick`
  (params (DeltaSeconds :type "Float (single-precision)"))
  (if (`self.IsCompleted`)
    (`/Engine/EditorBlueprintResources/StandardMacros.DoOnce` false
      (:`Completed`
        ; When the mission is completed, display "You Win!", wait for a few seconds, then navigate to the main menu.
        (bind _foundwidgets (`WidgetBlueprintLibrary.GetAllWidgetsOfClass` "/Game/Pangaea/UI/HUD.HUD_C"))
        (set `/Game/Pangaea/UI/HUD.GameOverText` "You Win!" (`|GetArrayItem` _foundwidgets))
        (`KismetSystemLibrary.Delay` 10.0)
        (`GameplayStatics.OpenLevel` "MainMenu")))
    (else
      ; Loop through the objectives. Break if an incomplete one is found and activate it. Otherwise, keep IsCompleted as true.
      (set `self.IsCompleted` true)
      (for _array_element (`self.Objectives`) :!label _label
        (if (not (`/Game/Pangaea/Mission/BP_Objective.IsCompleted` _array_element))
          (set `/Game/Pangaea/Mission/BP_Objective.IsActive` true _array_element)
          (set `self.IsCompleted` false)
          (`self.BreakForLoop`))))))

(event `BreakForLoop`
  ; Loop through the objectives. Break if an incomplete one is found and activate it. Otherwise, keep IsCompleted as true.
  (goto _label :!via `Break`))

(fn `UserConstructionScript`)