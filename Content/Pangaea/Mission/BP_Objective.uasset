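; BP_Objective is a mission objective actor that completes once every actor in its tracked Actors list is no longer valid.
; While active, its first overlap with BP_Hero prints the Title and shows it through the HUD1 widget's ShowMissionOrObjective.
; Each Tick scans Actors, stops at the first valid one, then derives IsCompleted and clears IsActive when none remain.
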(event `self.ReceiveBeginPlay`
  (`KismetSystemLibrary.PrintString` "Objective1"))

(event `self.ReceiveActorBeginOverlap`
  (params (OtherActor :type "Actor Object Reference"))
  (bind _title (`self.Title`))
  (if (`self.IsActive`)
    (cast `/Game/Pangaea/Characters/Hero/BP_Hero` OtherActor)
    (`/Engine/EditorBlueprintResources/StandardMacros.DoOnce` false
      (:`Completed`
        (`KismetSystemLibrary.PrintString` _title true true (struct :`G` 0.66 :`B` 1.0 :`A` 1.0) 15.0)
        (bind _foundwidgets (`WidgetBlueprintLibrary.GetAllWidgetsOfClass` "/Game/Pangaea/UI/HUD1.HUD1_C"))
        (`/Game/Pangaea/UI/HUD1.ShowMissionOrObjective` (`|GetArrayItem` _foundwidgets) _title)))))

(event `self.ReceiveTick`
  (params (DeltaSeconds :type "Float (single-precision)"))
  (bind _actors (`self.Actors`))
  (if (`self.IsActive`)
    (for (_array_element _array_index) _actors :!label _label
      (bind _returnvalue (`KismetSystemLibrary.IsValid` _array_element))
      ; Still has an active actor, break the loop.
      (if _returnvalue
        (`self.BreakForLoop`)))
    (bind _returnvalue_2 (and (not _returnvalue) (>= _array_index (- (`KismetArrayLibrary.Array_Length` _actors) 1))))
    ; Set IsCompleted and IsActive
    (set `self.IsCompleted` _returnvalue_2)
    (set `self.IsActive` (not _returnvalue_2))))

(event `BreakForLoop`
  (goto _label :!via `Break`))

(fn `UserConstructionScript`)