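; BP_Loop is a Blueprint that demonstrates a while loop by printing a countdown.
; On BeginPlay it sets X to 20, then decrements X and prints its value each iteration until it reaches zero, followed by a completion message.
; The overlap and tick events are disabled placeholders, and the construction script is empty.
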(event `self.ReceiveBeginPlay`
  (set `self.X` 20)
  (while (> (`self.X`) 0)
    (bind _output_get (set `self.X` (- (`self.X`) 1)))
    (`KismetSystemLibrary.PrintString` (`KismetStringLibrary.Concat_StrStr` "x = " (`KismetStringLibrary.Conv_IntToString` _output_get))))
  (`KismetSystemLibrary.PrintString` "a is 0 now"))

(fn `UserConstructionScript`)