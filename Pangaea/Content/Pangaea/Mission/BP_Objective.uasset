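; BP_Objective is a mission objective actor that announces itself to the hero and tracks completion through a list of actors.
; While active, its first overlap with BP_Hero prints the Title on screen.
; While active, Tick polls Actors and marks the objective completed when none remain valid.
; Tick then copies IsCompleted into IsActive, so the objective deactivates while any listed actor is still valid.
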(event `self.ReceiveActorBeginOverlap`
  (params (OtherActor :type "Actor Object Reference"))
  (if (`self.IsActive`)
    (cast `/Game/Pangaea/Characters/Hero/BP_Hero` OtherActor)
    (`/Engine/EditorBlueprintResources/StandardMacros.DoOnce` false
      (:`Completed`
        (`KismetSystemLibrary.PrintString` (`self.Title`) true true (struct :`G` 0.66 :`B` 1.0 :`A` 1.0) 15.0)))))

(event `self.ReceiveTick`
  (params (DeltaSeconds :type "Float (single-precision)"))
  (if (`self.IsActive`)
    (set `self.IsCompleted` true)
    (for _array_element (`self.Actors`)
      (if (`KismetSystemLibrary.IsValid` _array_element)
        (set `self.IsCompleted` false)))
    (set `self.IsActive` (`self.IsCompleted`))))

(fn `UserConstructionScript`)