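; BP_Hero is the player-controlled hero character, with movement, camera look and a sword attack.
; On BeginPlay it resets the AB_Hero animation state and attaches a spawned BP_Sword to the right-hand socket.
; Input actions drive turning with forward-only movement, spring arm rotation with clamped pitch, and attacks that switch AnimState from idle.
; Tick feeds normalized movement speed to the anim instance for locomotion.
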(event `self.ReceiveBeginPlay`
  (`|ExecutionSequence`
    (:`then_0`
      (bind _asab_hero (cast `/Game/Pangaea/Characters/Hero/AB_Hero` (`SkeletalMeshComponent.GetAnimInstance` (`self.Mesh`))))
      (set `/Game/Pangaea/Characters/Hero/AB_Hero.AnimState` 0 _asab_hero))
    (:`then_1`
      (bind _returnvalue (`|SpawnActorFromClass` "/Game/Pangaea/Weapons/Sword/BP_Sword.BP_Sword_C" (`self.GetTransform`) "AlwaysSpawn" "MultiplyWithRoot" null null))
      (`self.K2_AttachToComponent` _returnvalue (`self.Mesh`) "hand_rSocket" "SnapToTarget" "SnapToTarget" "SnapToTarget" true))))

(event `EnhancedInput|/Game/Pangaea/Input/Actions/Action_Attack`
  (params (ActionValue :type Boolean) (ElapsedSeconds :type "Float (double-precision)") (TriggeredSeconds :type "Float (double-precision)") (InputAction :type "InputAction Object Reference" :default "/Game/Pangaea/Input/Actions/Action_Attack.Action_Attack"))
  (:`Triggered`
    (`self.Attack`)))

(event `EnhancedInput|/Game/Pangaea/Input/Actions/Action_Move`
  (params (ActionValue :type "Vector2D Structure") (ElapsedSeconds :type "Float (double-precision)") (TriggeredSeconds :type "Float (double-precision)") (InputAction :type "InputAction Object Reference" :default "/Game/Pangaea/Input/Actions/Action_Move.Action_Move"))
  (bind (_x _y) (`KismetMathLibrary.BreakVector2D` ActionValue))
  (:`Triggered`
    (`self.MoveHero` _x _y)))

(event `EnhancedInput|/Game/Pangaea/Input/Actions/Action_Hero_Look`
  (params (ActionValue :type "Vector2D Structure") (ElapsedSeconds :type "Float (double-precision)") (TriggeredSeconds :type "Float (double-precision)") (InputAction :type "InputAction Object Reference" :default "/Game/Pangaea/Input/Actions/Action_Hero_Look.Action_Hero_Look"))
  (bind (_x _y) (`KismetMathLibrary.BreakVector2D` ActionValue))
  (:`Triggered`
    (`self.HeroLook` _x _y)))

(event `self.ReceiveTick`
  (params (DeltaSeconds :type "Float (single-precision)"))
  (bind _returnvalue (`self.GetMovementComponent`))
  ; Sync Locomotion Animation
  (set `/Game/Pangaea/Characters/Hero/AB_Hero.Speed` (/ (`KismetMathLibrary.VSize` (`NavMovementInterface.GetVelocityForNavMovement` _returnvalue)) (`NavMovementInterface.GetMaxSpeedForNavMovement` _returnvalue)) (`self.GetAnimInst`)))

(fn `Attack`
  (bind _animinst (`self.GetAnimInst`))
  (if (== (`/Game/Pangaea/Characters/Hero/AB_Hero.AnimState` _animinst) 0)
    (set `/Game/Pangaea/Characters/Hero/AB_Hero.AnimState` 1 _animinst)))

(fn `GetAnimInst`
  (returns (AnimInst :type "/Game/Pangaea/Characters/Hero/AB_Hero Object Reference"))
  (bind _asab_hero (cast `/Game/Pangaea/Characters/Hero/AB_Hero` (`SkeletalMeshComponent.GetAnimInstance` (`self.Mesh`))))
  (return _asab_hero))

(fn `HeroLook`
  (params (`X Axis` :type "Float (double-precision)") (`Y Axis` :type "Float (double-precision)"))
  (bind _springarm (`self.SpringArm`))
  ; Rotating the camera view
  (`SceneComponent.K2_AddRelativeRotation` (`self.SpringArm`) (`KismetMathLibrary.MakeRotator` 0.0 `X Axis` `Y Axis`) false false)
  ; Clamp the up/down the spring arm rotation within -30 and 30 degrees
  (`SceneComponent.K2_SetRelativeRotation` _springarm (`KismetMathLibrary.MakeRotator` (.roll (`SceneComponent.RelativeRotation` _springarm)) (`KismetMathLibrary.FClamp` (.pitch (`SceneComponent.RelativeRotation` _springarm)) -30.0 30.0) (.yaw (`SceneComponent.RelativeRotation` _springarm))) false false))

(fn `MoveHero`
  (params (`X Aixs` :type "Float (double-precision)") (`Y Axis` :type "Float (double-precision)"))
  ; Check if Y Axis value is greater than 0. Only allows player to move forward
  (if (>= `Y Axis` 0.0)
    ; Move forward
    (`self.AddControllerYawInput` `X Aixs`)
    (`self.AddMovementInput` (`self.GetActorForwardVector`) (+ (`KismetMathLibrary.Abs` `X Aixs`) `Y Axis`))))

(fn `UserConstructionScript`)