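; BP_Warrok is an AI enemy character that spawns a BP_Hammer, senses the hero and reacts to damage.
; Perception of a BP_Hero writes the PlayerTarget blackboard key; the clearing node is unwired.
; Damage in certain AB_Warrok animation states lowers Health, stops movement and sets a hit or death AnimState, with delayed destruction of weapon and actor on death.
; Hammer socket attachment and Health initialisation are also unwired, so never run.
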(event `self.ReceiveBeginPlay`
  (bind _returnvalue (`|SpawnActorFromClass` "/Game/Pangaea/Weapons/Hammer/BP_Hammer.BP_Hammer_C" (`self.GetTransform`) "Undefined" "MultiplyWithRoot" null null)))

(event `self.AIPerception.OnTargetPerceptionInfoUpdated`
  (params (UpdateInfo :type "ActorPerceptionUpdateInfo Structure (by ref)"))
  (bind (_targetid _target _stimulus) (break `ActorPerceptionUpdateInfo` UpdateInfo))
  (cast `/Game/Pangaea/Characters/Hero/BP_Hero` _target)
  (if (`.bSuccessfullySensed` (break `AIStimulus` _stimulus))
    (`BlackboardComponent.SetValueAsObject` (`AIBlueprintHelperLibrary.GetBlackboard` (`AIBlueprintHelperLibrary.GetAIController` self)) "PlayerTarget" null)))

(event `self.ReceiveAnyDamage`
  (params (Damage :type "Float (single-precision)") (DamageType :type "DamageType Object Reference") (InstigatedBy :type "Controller Object Reference") (DamageCauser :type "Actor Object Reference"))
  (bind _asab_warrok (cast `/Game/Pangaea/Characters/Warrok/AB_Warrok` (`SkeletalMeshComponent.GetAnimInstance` (`self.Mesh`))))
  (if true
    (bind _animstate (`/Game/Pangaea/Characters/Warrok/AB_Warrok.AnimState` _asab_warrok))
    (if (or (or (== _animstate 0) (== _animstate 11)) (== _animstate 12))
      (bind _output_get (set `self.Health` (- (`self.Health`) Damage)))
      (if (>= _output_get 0)
        (bind _returnvalue (`AIBlueprintHelperLibrary.GetAIController` null))
        (`Controller.StopMovement` _returnvalue)
        (set `self.AnimState` 2)
        (else
          (bind _returnvalue_2 (`AIBlueprintHelperLibrary.GetAIController` null))
          (`Controller.StopMovement` _returnvalue_2)
          (set `self.AnimState` 3)
          (`KismetSystemLibrary.Delay` 5.0)
          (`self.K2_DestroyActor` (`self.Weapon`))
          (`self.K2_DestroyActor`))))))

(fn `UserConstructionScript`)