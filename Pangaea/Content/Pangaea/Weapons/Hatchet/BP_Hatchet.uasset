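; BP_Hatchet is a melee weapon actor carried by the boss (Warrok) that damages whatever it hits during attacks.
; On actor overlap it ignores its attach parent and casts that parent to BP_Boss.
; It applies fixed damage only while the boss's anim instance AnimState is one of two attack states, checked against hard-coded numeric values.
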(event `self.ReceiveActorBeginOverlap`
  (params (OtherActor :type "Actor Object Reference"))
  (bind _returnvalue (`self.GetAttachParentActor`))
  ; Check if it is not Warrok itself
  (if (!= OtherActor _returnvalue)
    (bind _asbp_boss (cast `/Game/Pangaea/Characters/Boss/BP_Boss` _returnvalue))
    (bind _animstate (`/Game/Pangaea/Characters/Boss/AB_Boss.AnimState` (`/Game/Pangaea/Characters/Boss/BP_Boss.GetAnimInst` _asbp_boss)))
    ; Check if is attacking
    (if (or (== _animstate 11) (== _animstate 12))
      (`GameplayStatics.ApplyDamage` OtherActor 100.0 null self))))

(fn `UserConstructionScript`)